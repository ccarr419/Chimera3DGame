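; Waystone is an interactable checkpoint that sets the player's respawn point when activated.
; A box overlap enables input while the player is nearby, and the E key activates the waystone only once.
; Activation toggles the particles and spotlight that were hidden at BeginPlay, then stores its Scene transform as PlayerSpawnLocation in FirstPersonGameMode.
; It also shows a "Waypoint Set" DropDownText widget.
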(event OnComponentBeginOverlap(Box)
  (params (OverlappedComponent :type Primitive%20Component%20Object%20Reference) (OtherActor :type Actor%20Object%20Reference) (OtherComp :type Primitive%20Component%20Object%20Reference) (OtherBodyIndex :type Integer) (bFromSweep :type Boolean) (SweepResult :type Hit%20Result%20Structure%20%28by%20ref%29))
  ;[1 1 1] Enable input on entry, disable on leave
  (Input|EnableInput (Game|GetPlayerController 0)))

(event OnComponentEndOverlap(Box)
  (params (OverlappedComponent :type Primitive%20Component%20Object%20Reference) (OtherActor :type Actor%20Object%20Reference) (OtherComp :type Primitive%20Component%20Object%20Reference) (OtherBodyIndex :type Integer))
  ;[1 1 1] Enable input on entry, disable on leave
  (Input|DisableInput (Game|GetPlayerController 0)))

(event EventBeginPlay
  ;[1 1 1] Hide particle and light on spawn
  (Components|Activation|ToggleActive (Variables|Default|GetBlueMagic))
  (Rendering|ToggleVisibility (Variables|Default|GetSpotLight) false)
  (Components|Activation|ToggleActive (Variables|Default|GetFire)))

(event Collision|EventActorBeginOverlap
  (params (OtherActor :type Actor%20Object%20Reference)))

(event EventTick
  (params (DeltaSeconds :type Float%20%28single-precision%29)))

(event Input|KeyboardEvents|E
  (params (Key :type Key%20Structure :default "AnyKey"))
  ;[1 1 1] If Waypoint is not active...
  (:Pressed
    (if (not (Variables|Default|GetIsActive))
      ;[1 1 1] Toggle particle and light on
      (Components|Activation|ToggleActive (Variables|Default|GetBlueMagic))
      (Rendering|ToggleVisibility (Variables|Default|GetSpotLight) false)
      (Components|Activation|ToggleActive (Variables|Default|GetFire))
      (Variables|Default|SetIsActive true)
      (Development|PrintString "Activated!")
      ;[1 1 1] Set player respawn location upon activation
      (bind _asfirst_person_game_mode (Utilities|Casting|CastToFirstPersonGameMode (Game|GetGameMode)))
      (Variables|/Game/FirstPersonBP/Blueprints/FirstPersonGameMode.FirstPersonGameMode_C|SetPlayerSpawnLocation _asfirst_person_game_mode (Transformation|GetWorldTransform (Variables|Default|GetScene)))
      ;[1 1 1] "Waypoint Set" printed to screen widget
      (bind _returnvalue (UserInterface|CreateWidget "/Game/UI/DropDownText.DropDownText_C" (Game|GetPlayerController 0)))
      (UserInterface|Viewport|AddtoViewport _returnvalue 0)
      (Default|PlayAnim _returnvalue "Waypoint Set"))))

(fn ConstructionScript)