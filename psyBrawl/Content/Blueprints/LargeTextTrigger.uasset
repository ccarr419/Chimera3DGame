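; LargeTextTrigger is a one-shot trigger actor that shows a drop-down text message when the FirstPersonCharacter overlaps it.
; On the first player overlap, it creates a DropDownText widget, passes it TextToSet, adds it to the viewport and sets Triggered to block repeats.
; If AddsToPuzzleComplete is set, it also increments the PuzzlesComplete count in psyBrawlGameInstance.
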(event EventBeginPlay)

(event Collision|EventActorBeginOverlap
  (params (OtherActor :type Actor%20Object%20Reference))
  ;[1 1 1] Only trigger if collider is player
  (Utilities|Casting|CastToFirstPersonCharacter OtherActor)
  ;[1 1 1] If still active...
  (if (not (Variables|Default|GetTriggered))
    ;[1 1 1] Create text
    (bind _returnvalue (UserInterface|CreateWidget "/Game/UI/DropDownText.DropDownText_C" (Game|GetPlayerController 0)))
    ;[1 1 1] Text set
    (Variables|/Game/UI/DropDownText.DropDownText_C|SetSetText _returnvalue (Variables|Default|GetTextToSet))
    ;[1 1 1] Add to UI
    (UserInterface|Viewport|AddtoViewport _returnvalue 0)
    ;[1 1 1] Set inactive
    (Variables|Default|SetTriggered true)
    ;[1 1 1] If set as a puzzle complete, increment the number of puzzles complete for the level
    (if (Variables|Default|GetAddsToPuzzleComplete)
      (bind _aspsy_brawl_game_instance (Utilities|Casting|CastTopsyBrawlGameInstance (Game|GetGameInstance)))
      (bind _result (Math|Integer|IncrementInt (Variables|/Game/FirstPersonBP/Blueprints/psyBrawlGameInstance.psyBrawlGameInstance_C|GetPuzzlesComplete _aspsy_brawl_game_instance))
        (:%20%20
          (Variables|/Game/FirstPersonBP/Blueprints/psyBrawlGameInstance.psyBrawlGameInstance_C|SetPuzzlesComplete _aspsy_brawl_game_instance _result))))))

(event EventTick
  (params (DeltaSeconds :type Float%20%28single-precision%29)))

(fn ConstructionScript)