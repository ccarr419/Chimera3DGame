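; Trigger actor that plays an end-of-game cutscene, then shows the victory screen and returns to the MenuIsland level.
; Any actor overlap plays the CutsceneToPlay level sequence, disables player input and removes all widgets, with no filter or re-trigger guard.
; A timer matching the sequence length, rather than a finish event, calls SequenceComplete, which displays VictoryUI and opens the menu after a short delay.
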(event Custom|SequenceComplete
  (bind _returnvalue (UserInterface|CreateWidget "/Game/UI/VictoryUI.VictoryUI_C" (Game|GetPlayerController 0)))
  (UserInterface|Viewport|AddtoViewport _returnvalue 0)
  (Utilities|FlowControl|Delay 3.0)
  (Game|OpenLevel(byName) "MenuIsland"))

(event EventBeginPlay)

(event Collision|EventActorBeginOverlap
  (params (OtherActor :type Actor%20Object%20Reference))
  (bind _returnvalue (Game|GetPlayerController 0))
  ;[1 1 1] On collision, play referenced level sequence
  (bind _returnvalue_2 (Sequencer|Player|CreateLevelSequencePlayer (Variables|Default|GetCutsceneToPlay)))
  (Sequencer|Player|Play _returnvalue_2 :!class /Script/MovieScene.MovieSceneSequencePlayer)
  ;[1 1 1] Stop movement and remove hud elements
  (Input|DisableInput _returnvalue _returnvalue)
  (Viewport|RemoveAllWidgets)
  (Utilities|Time|SetTimerbyEvent (delegate Custom|SequenceComplete) (Class|MovieSceneSequencePlayer|GetLength _returnvalue_2)))

(event EventTick
  (params (DeltaSeconds :type Float%20%28single-precision%29)))

(fn ConstructionScript)